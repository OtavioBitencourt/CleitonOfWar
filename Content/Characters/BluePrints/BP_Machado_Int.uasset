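; BP_Machado_Int is an axe pickup that equips the player character when touched.
; When the player overlaps its Sphere, it sets the BP_ThirdPersonCharacter's State enum and unhides the BruteAxe component already on that character.
; It then sets Equipped on the mesh's Cleiton_AnimBP and destroys itself, so no axe actor is spawned or attached.
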(event OnComponentBeginOverlap(Sphere)
  (params (OverlappedComponent :type Primitive%20Component%20Object%20Reference) (OtherActor :type Actor%20Object%20Reference) (OtherComp :type Primitive%20Component%20Object%20Reference) (OtherBodyIndex :type Integer) (bFromSweep :type Boolean) (SweepResult :type Hit%20Result%20Structure%20%28by%20ref%29))
  (bind _returnvalue (Game|GetPlayerCharacter 0))
  ;[0.9793 1 0.8402] Equipa o machado
  (if (== OtherActor _returnvalue)
    (bind _asbp_third_person_character (Utilities|Casting|CastToBP_ThirdPersonCharacter _returnvalue))
    (Variables|/Game/ThirdPerson/Blueprints/BP_ThirdPersonCharacter.BP_ThirdPersonCharacter_C|SetState _asbp_third_person_character "NewEnumerator0")
    (Development|SetHiddeninGame (Variables|/Game/ThirdPerson/Blueprints/BP_ThirdPersonCharacter.BP_ThirdPersonCharacter_C|GetBrute_Axe _asbp_third_person_character) false false)
    (bind _ascleiton_anim_bp (Utilities|Casting|CastToCleiton_AnimBP (Components|SkeletalMesh|GetAnimInstance (Variables|/Script/Engine.Character|GetMesh _asbp_third_person_character))))
    (Variables|/Game/Characters/Animations/Cleiton/Cleiton_AnimBP.Cleiton_AnimBP_C|Setequipped _ascleiton_anim_bp true)
    (Actor|DestroyActor)))

(fn ConstructionScript)