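; Enemy character Blueprint that chases the player and attacks in melee.
; After a short random delay at BeginPlay, it focuses the player and loops AI MoveTo, retrying after a pause on failure.
; On arrival it plays an attack montage, applies delayed damage if the player overlaps its sphere and it is alive, then resumes chasing.
; Any damage received marks it dead and unpossesses its AI controller, stopping the loop.
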(event Custom|MoveToPlayer
  ;[1 0.8305 0.3106] Movimentação
  ;;[1 1 1] Verifica se o AIController é válido
  (Utilities|IsValid (AI|GetAIController self)
    (:Is%20Valid
      ;;[1 1 1] Faz o inimigo se mover
      (AI|AIMoveTo self "0, 0, 0" (Game|GetPlayerCharacter 0) 5.0 false
        (:OnSuccess
          ;;[1 1 1] Executa a animação de ataque
          (bind _returnvalue (Animation|PlayAnimMontage "/Game/Characters/Animations/Enemy/Enemy_Attack_Root_Anim_Montage.Enemy_Attack_Root_Anim_Montage" 1.0 "None"))
          (Utilities|FlowControl|Sequence
            (:then_0
              (Utilities|FlowControl|Delay 1.0)
              (if (Collision|IsOverlappingActor (Variables|Default|GetSphere) (Game|GetPlayerCharacter 0) :!class /Script/Engine.PrimitiveComponent)
                ;;[1 1 1] Ativa somente se o inimigo não estiver morto
                (if (not (Variables|Default|GetDead))
                  ;;[1 1 1] Aplica dano ao jogador
                  (Game|Damage|ApplyDamage (Game|GetPlayerCharacter 0) 1.0 0 0))))
            (:then_1
              ;;[1 1 1] Reinicia a movimentação
              (Utilities|FlowControl|Delay _returnvalue)
              (CallFunction|MovetoPlayer :!label _label))))
        (:OnFail
          (Utilities|FlowControl|Delay 2.0)
          (goto _label))))))

(event EventBeginPlay
  ;[1 0.8305 0.3106] Movimentação
  ;;[1 1 1] Configura o Foco no Player
  (AI|SetFocus (AI|GetAIController self) (Game|GetPlayerCharacter 0))
  ;;[1 1 1] Gera um atraso para iniciar a movimentação
  (Utilities|FlowControl|Delay (Math|Random|RandomFloatinRange 0.0 1.0))
  ;;[1 1 1] Verifica se o AIController é válido
  (Utilities|IsValid (AI|GetAIController self)
    (:Is%20Valid
      ;;[1 1 1] Faz o inimigo se mover
      (AI|AIMoveTo self "0, 0, 0" (Game|GetPlayerCharacter 0) 5.0 false
        (:OnSuccess
          ;;[1 1 1] Executa a animação de ataque
          (bind _returnvalue (Animation|PlayAnimMontage "/Game/Characters/Animations/Enemy/Enemy_Attack_Root_Anim_Montage.Enemy_Attack_Root_Anim_Montage" 1.0 "None"))
          (Utilities|FlowControl|Sequence
            (:then_0
              (Utilities|FlowControl|Delay 1.0)
              (if (Collision|IsOverlappingActor (Variables|Default|GetSphere) (Game|GetPlayerCharacter 0) :!class /Script/Engine.PrimitiveComponent)
                ;;[1 1 1] Ativa somente se o inimigo não estiver morto
                (if (not (Variables|Default|GetDead))
                  ;;[1 1 1] Aplica dano ao jogador
                  (Game|Damage|ApplyDamage (Game|GetPlayerCharacter 0) 1.0 0 0))))
            (:then_1
              ;;[1 1 1] Reinicia a movimentação
              (Utilities|FlowControl|Delay _returnvalue)
              (CallFunction|MovetoPlayer :!label _label))))
        (:OnFail
          (Utilities|FlowControl|Delay 2.0)
          (goto _label))))))

(event Game|Damage|EventAnyDamage
  (params (Damage :type Float%20%28single-precision%29) (DamageType :type Damage%20Type%20Object%20Reference) (InstigatedBy :type Controller%20Object%20Reference) (DamageCauser :type Actor%20Object%20Reference))
  (bind _self self)
  (bind _returnvalue (AI|GetAIController _self))
  ;[1 0.3078 0.198] AnyDamage
  (Variables|Default|SetDead true)
  (Utilities|IsValid _returnvalue
    (:Is%20Valid
      (Pawn|UnPossess _returnvalue))))

(fn ConstructionScript)